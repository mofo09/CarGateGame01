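; SphereMap_BP is a background sphere-map actor with Front, Mid, Back and Clouds components, whose overall size can grow or shrink at runtime.
; Its only live logic is the AddToSphereScale event, which adds a given vector to the root's current world scale.
; Nodes that would zero each layer's relative scale are left unconnected, and the construction script is empty.
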(event `AddToSphereScale`
  (params (vector :type "Vector Structure"))
  (bind _defaultsceneroot (`self.DefaultSceneRoot`))
  (`SceneComponent.SetWorldScale3D` _defaultsceneroot (+ (`SceneComponent.K2_GetComponentScale` _defaultsceneroot) vector)))

(fn `UserConstructionScript`)